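; BP_FPCharacter is a character Blueprint that detects a minion in front of it and signals text visibility for that target.
; Each Tick it traces a short distance forward for Pawn objects, acting only when the hit state changes.
; On a change it fires the SetText dispatcher with visibility and the cast BP_Minion, then stores the target.
; A separate UI reference keeps the last valid minion until ResetTargetMinion clears both.
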(event EventBeginPlay
  (Variables|Default|SetIsTextEnabled false))

(event Collision|EventActorBeginOverlap
  (params (OtherActor :type Actor%20Object%20Reference)))

(event EventTick
  (params (DeltaSeconds :type Float%20%28single-precision%29))
  (bind _returnvalue (Transformation|GetActorLocation))
  (bind (_outhit _returnvalue_2) (Collision|LineTraceForObjects _returnvalue (+ _returnvalue (* (Math|Vector|GetForwardVector (Transformation|GetActorRotation)) 2e+02)) (Utilities|Array|MakeArray "ObjectTypeQuery3") false 0 "None"))
  (if (Class|KismetMathLibrary|XORBoolean _returnvalue_2 (Variables|Default|GetIsTextEnabled))
    (bind _asbp_minion_1 (Utilities|Casting|CastToBP_Minion (.HitActor (Collision|BreakHitResult _outhit)))
      (:then
        _)
      (:CastFailed
        _))
    (Default|CallSetTextDispatcher _returnvalue_2 _asbp_minion_1)
    (Variables|Default|SetIsTextEnabled _returnvalue_2)
    (bind _output_get (Variables|Default|SetTargetMinion _asbp_minion_1))
    (if (Utilities|IsValid _output_get)
      (CallFunction|SaveTargetMinionforUI))))

(fn ConstructionScript)

(fn ResetTargetMinion
  (Variables|Default|SetTargetMinion 0)
  (Variables|Default|SetTargetMinionForUI 0))

(fn SaveTargetMinionforUI
  (Variables|Default|SetTargetMinionForUI (Variables|Default|GetTargetMinion)))